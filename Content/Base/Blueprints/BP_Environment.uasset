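; Environment bridge actor that exposes Ultra Dynamic Sky and Weather time and weather values to the game.
; On BeginPlay it caches the weather actor, found by interface, only if exactly one exists.
; Time setter and getter convert between game time and sky TimeOfDay.
; Getters return scaled fog, rain and cached fog-plane values, or zero without a weather actor; IsEffectPlaying is a stub returning false.
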(event `self.ReceiveBeginPlay`
  (bind _outactors (`GameplayStatics.GetAllActorsWithInterface` "/Game/BaseNoGit/ThirdParty/UltraDynamicSky/Blueprints/Weather_Effects/System/Ultra_Dynamic_Weather_Interface.Ultra_Dynamic_Weather_Interface_C"))
  (if (== (`KismetArrayLibrary.Array_Length` _outactors) 1)
    (bind _asultra_dynamic_weather (cast `/Game/BaseNoGit/ThirdParty/UltraDynamicSky/Blueprints/Ultra_Dynamic_Weather` (`|GetArrayItem` _outactors)))
    (set `self.UDS` _asultra_dynamic_weather)))

(event `self.SetGameTime`
  (params (InTime :type "Float (single-precision)") (InTimeFactor :type "Float (single-precision)"))
  (set `/Game/BaseNoGit/ThirdParty/UltraDynamicSky/Blueprints/Ultra_Dynamic_Sky.Time of Day` (* InTime 0.027778) (`/Game/BaseNoGit/ThirdParty/UltraDynamicSky/Blueprints/Ultra_Dynamic_Weather.UltraDynamicSky` (`self.UDS`))))

(fn `GetFogDensity`
  (returns (ReturnValue :type "Float (single-precision)"))
  (bind _uds (`self.UDS`))
  (`/Engine/EditorBlueprintResources/StandardMacros.IsValid` _uds
    (:`Is Valid`
      (bind (_cloud_coverage _wind_intensity _rain _snow _dust _fog) (`/Game/BaseNoGit/ThirdParty/UltraDynamicSky/Blueprints/Ultra_Dynamic_Weather.Get Local Weather State Values` _uds))
      (return (/ _fog 10.0)))
    (:`Is Not Valid`
      (return 0.0))))

(fn `GetFogPlane`
  (returns (ReturnValue :type "Float (single-precision)"))
  (bind _uds (`self.UDS`))
  (`/Engine/EditorBlueprintResources/StandardMacros.IsValid` _uds
    (:`Is Valid`
      (bind _value (`/Game/BaseNoGit/ThirdParty/UltraDynamicSky/Blueprints/Ultra_Dynamic_Sky.Get Cached Float` (`/Game/BaseNoGit/ThirdParty/UltraDynamicSky/Blueprints/Ultra_Dynamic_Weather.UltraDynamicSky` _uds) "NewEnumerator57"))
      (return (/ _value 100.0)))
    (:`Is Not Valid`
      (return 0.0))))

(fn `GetGameTime`
  (returns (ReturnValue :type "Float (single-precision)"))
  (bind _uds (`self.UDS`))
  (`/Engine/EditorBlueprintResources/StandardMacros.IsValid` _uds
    (:`Is Valid`
      (return (/ (`/Game/BaseNoGit/ThirdParty/UltraDynamicSky/Blueprints/Ultra_Dynamic_Sky.Time of Day` (`/Game/BaseNoGit/ThirdParty/UltraDynamicSky/Blueprints/Ultra_Dynamic_Weather.UltraDynamicSky` _uds)) 0.027778)))
    (:`Is Not Valid`
      (return 0.0))))

(fn `GetRainDensity`
  (returns (ReturnValue :type "Float (single-precision)"))
  (bind _uds (`self.UDS`))
  (`/Engine/EditorBlueprintResources/StandardMacros.IsValid` _uds
    (:`Is Valid`
      (bind (_cloud_coverage _wind_intensity _rain) (`/Game/BaseNoGit/ThirdParty/UltraDynamicSky/Blueprints/Ultra_Dynamic_Weather.Get Local Weather State Values` _uds))
      (return (/ _rain 10.0)))
    (:`Is Not Valid`
      (return 0.0))))

(fn `IsEffectPlaying`
  (returns (ReturnValue :type Boolean))
  (return false))

(fn `UserConstructionScript`)